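; BP_SoundMaster plays a tutorial sound and spawns spectrum visualization actors as it plays.
; PlayTutorialSound starts the audio and binds its playback-percent event, which converts progress to seconds to sample normalized Constant-Q analysis on channel 0.
; The loop over those values feeds BP_AudioElement spawns at the root, with Z scale driven by magnitude.
; A Delay inside the loop means spawns do not occur once per value.
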(event `self.ReceiveBeginPlay`)

(event `PlayTutorialSound`
  (`AudioComponent.SetSound` (`self.Audio`) (`self.New Sound`))
  (set `self.Duration` (`SoundBase.Duration` (`self.New Sound`)))
  (add `AudioComponent.OnAudioPlaybackPercent` (`self.Audio`) (delegate `PlaybackChange`))
  (`AudioComponent.Play` (`self.Audio`) 0.0))

(event `PlaybackChange`
  (params (PlayingSoundWave :type "SoundWave Object Reference") (PlaybackPercent :type "Float (single-precision)"))
  (set `self.PlayedTime` (* PlaybackPercent (`self.Duration`)))
  (for _array_element (`ConstantQNRT.GetNormalizedChannelConstantQAtTime` (`self.Constant_Ref`) (`self.PlayedTime`) 0)
    (`KismetSystemLibrary.Delay` 0.1)
    (`|SpawnActorFromClass` "/Game/VocSimVr/Blueprints/BP_AudioElement.BP_AudioElement_C" (`KismetMathLibrary.MakeTransform` (`SceneComponent.K2_GetComponentLocation` (`self.DefaultSceneRoot`)) (struct) (`KismetMathLibrary.MakeVector` 0.01 0.05 (* _array_element 3.0))) "Undefined" "MultiplyWithRoot" null null)))

(fn `UserConstructionScript`)